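; First-person player character with stand/crouch/prone stances, sprinting, interface-based interaction, a battery flashlight, a pickaxe and a gas mask widget.
; Stance functions set state and speed, sphere-tracing for headroom before rising, while Tick interpolates capsule height and sprint FOV.
; A looping timer, paused while the flashlight is off, handles battery drain.
; Pickaxe swings use a timeline and spawn MF_Wall; damage reduces health, disabling movement and input at death.
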(event Custom|BatteryDrain
  ;[1 1 1] Flashlight
  (if (and (Variables|Default|GetFlashlightOn) (> (Variables|Default|GetBatteryPercent) 0.0))
    (Variables|Default|SetBatteryPercent (- (Variables|Default|GetBatteryPercent) 0.03))
    (if (<= (Variables|Default|GetBatteryPercent) 0.0)
      (CallFunction|ShutdownFlashlight))))

(event Custom|ShutdownFlashlight
  ;[1 1 1] Flashlight
  (Rendering|SetVisibility (Variables|Default|GetFlashlight) false false)
  (Utilities|Time|PauseTimerbyHandle (Variables|Default|GetBatteryTimerHandle))
  (Variables|Default|SetFlashlightOn false))

(event Custom|BatteryRecharge
  ;[1 1 1] Flashlight
  (bind _output_get (Variables|Default|SetBatteryPercent (+ (Variables|Default|GetBatteryPercent) (Math|Random|RandomFloatinRange 15.0 6e+01))))
  (if (>= _output_get 1e+02)
    (Variables|Default|SetBatteryPercent 1e+02)))

(event Custom|PickUpPickaxe
  ;[1 1 1] Pickaxe
  (Rendering|SetVisibility (Variables|Default|GetPickaxe) true false)
  (Variables|Default|SetHasPickaxe true)
  (Variables|Default|SetPickaxeUsable true))

(event Custom|PickaxeUseAnimation
  (bind _pickaxe (Variables|Default|GetPickaxe))
  (bind _relativerotation (Variables|/Script/Engine.SceneComponent|GetRelativeRotation _pickaxe))
  ;[1 1 1] Pickaxe
  (Utilities|FlowControl|Sequence
    (:then_0
      (bind _pickaxemovement (Timeline|UsePickaxeTimeline PlayFromStart)
        (:Update
          (Transformation|SetRelativeRotation _pickaxe (Math|Rotator|MakeRotator (* _pickaxemovement 6e+01) (.pitch _relativerotation) (.yaw _relativerotation)) false false))
        (:Finished
          (Variables|Default|SetPickaxeUsable true))))
    (:then_1
      (Utilities|FlowControl|Delay 0.3)
      (Game|SpawnActorfromClass "/Game/Ziya/MF_Wall.MF_Wall_C" (Transformation|GetWorldTransform (Variables|Default|GetAxeHitLocation)) "AlwaysSpawn" "MultiplyWithRoot" 0 0))))

(event Custom|PickUpGasMask
  ;[1 1 1] PoisonGas
  (bind _returnvalue (UserInterface|CreateWidget "/Game/Ziya/Widgets/WBP_GasMask.WBP_GasMask_C"))
  (UserInterface|Viewport|AddtoViewport _returnvalue 0))

(event EventBeginPlay
  ;[1 1 1] BeginPlay
  (bind _returnvalue (Utilities|Time|SetTimerbyEvent (EventDispatchers|CreateEvent :!event Custom|BatteryDrain) 0.01 true))
  (bind _output_get (Variables|Default|SetBatteryTimerHandle _returnvalue))
  (Utilities|Time|PauseTimerbyHandle _output_get))

(event EventTick
  (params (DeltaSeconds :type Float%20%28single-precision%29))
  ;[1 1 1] Motion Smoothing
  (Utilities|FlowControl|Sequence
    (:then_0
      (CallFunction|SetCapsuleHalfHeight (Math|Interpolation|FInterpTo (Variables|/Script/Engine.CapsuleComponent|GetCapsuleHalfHeight (Variables|Collision|GetCapsuleComponent)) (Utilities|Select :Index (Variables|Default|GetE_StanceState) :NewEnumerator0 9e+01 :NewEnumerator1 6e+01 :NewEnumerator2 28.0) DeltaSeconds 7.0)))
    (:then_1
      (Camera|SetFieldOfView (Variables|Default|GetCamera) (Math|Interpolation|FInterpTo (Variables|/Script/Engine.CameraComponent|GetFieldOfView (Variables|Default|GetCamera)) (Math|Float|SelectFloat 135.0 1.2e+02 (Variables|Default|GetIsSprinting)) DeltaSeconds 3.0)))))

(event Game|Damage|EventAnyDamage
  (params (Damage :type Float%20%28single-precision%29) (DamageType :type Damage%20Type%20Object%20Reference) (InstigatedBy :type Controller%20Object%20Reference) (DamageCauser :type Actor%20Object%20Reference))
  ;[1 1 1] PoisonGas
  (if (and (not (Variables|Default|GetisDead?)) (Variables|Actor|GetbCanBeDamaged))
    (bind _output_get (Variables|Default|SetHealth (- (Variables|Default|GetHealth) Damage)))
    (if (<= (Variables|Default|GetHealth) 0.0)
      (Variables|Default|SetisDead? true)
      (Pawn|Components|CharacterMovement|DisableMovement (Variables|Character|GetCharacterMovement))
      (Input|DisableInput 0)
      (else
        (Development|PrintString (Utilities|String|ToString(Float) _output_get))))))

(event Input|ActionEvents|InputActionJump
  (params (Key :type Key%20Structure :default "None"))
  ;[1 1 1] CharacterMovement
  (:Pressed
    (switch Utilities|FlowControl|Switch|SwitchonE_PlayerStance (Variables|Default|GetE_StanceState)
      (:NewEnumerator0
        (Character|Jump)))))

(event Input|ActionEvents|InputActionCrouch
  (params (Key :type Key%20Structure :default "None"))
  ;[1 1 1] CharacterMovement
  (:Pressed
    (switch Utilities|FlowControl|Switch|SwitchonE_PlayerStance (Variables|Default|GetE_StanceState)
      (:NewEnumerator0
        (CallFunction|CrouchMode))
      (:NewEnumerator1
        (Utilities|FlowControl|FlipFlop
          (:A
            (CallFunction|ProneMode))
          (:B
            (CallFunction|StandMode))))
      (:NewEnumerator2
        (CallFunction|PronetoCrouchMode)))))

(event Input|ActionEvents|InputActionInteract
  (params (Key :type Key%20Structure :default "None"))
  ;[1 1 1] Interact
  (:Pressed
    (bind _array_element (Utilities|Array|ForEachLoopwithBreak (Collision|GetOverlappingActors "/Script/Engine.Actor" :!class /Script/Engine.Actor) :!label _label)
      (:LoopBody
        (if (Utilities|DoesObjectImplementInterface _array_element "/Game/Antonio/InteractInterface.InteractInterface_C")
          (Class|InteractInterface|Interact(Message) _array_element self)
          (goto _label Break))))))

(event Input|ActionEvents|InputActionFlashlight
  (params (Key :type Key%20Structure :default "None"))
  (bind _flashlight (Variables|Default|GetFlashlight))
  (bind _batterytimerhandle (Variables|Default|GetBatteryTimerHandle))
  ;[1 1 1] Flashlight
  (:Pressed
    (if (Variables|Default|GetFlashlightOn)
      (Rendering|SetVisibility _flashlight false false)
      (Utilities|Time|PauseTimerbyHandle _batterytimerhandle)
      (Variables|Default|SetFlashlightOn false)
      (elif (> (Variables|Default|GetBatteryPercent) 0.0)
        (Rendering|SetVisibility _flashlight true false)
        (Utilities|Time|UnpauseTimerbyHandle _batterytimerhandle)
        (Variables|Default|SetFlashlightOn true)))))

(event Input|ActionEvents|InputActionSprint
  (params (Key :type Key%20Structure :default "None"))
  (bind _charactermovement (Variables|Character|GetCharacterMovement))
  (bind _e_stancestate (Variables|Default|GetE_StanceState))
  ;[1 1 1] Player Stance
  (:Pressed
    (switch Utilities|FlowControl|Switch|SwitchonE_PlayerStance _e_stancestate
      (:NewEnumerator0
        (Variables|Default|SetIsSprinting true)
        (Variables|/Script/Engine.CharacterMovementComponent|SetMaxWalkSpeed _charactermovement 4.5e+02))))
  (:Released
    (switch Utilities|FlowControl|Switch|SwitchonE_PlayerStance _e_stancestate
      (:NewEnumerator0
        (Variables|Default|SetIsSprinting false)
        (Variables|/Script/Engine.CharacterMovementComponent|SetMaxWalkSpeed _charactermovement 3e+02)))))

(event Input|ActionEvents|InputActionPickaxe
  (params (Key :type Key%20Structure :default "None"))
  ;[1 1 1] Pickaxe
  (:Pressed
    (if (and (Variables|Default|GetPickaxeUsable) (Variables|Default|GetHasPickaxe))
      (Variables|Default|SetPickaxeUsable false)
      (CallFunction|PickaxeUseAnimation))))

(event Input|AxisEvents|InputAxisTurn
  (params (AxisValue :type Float%20%28single-precision%29))
  ;[1 1 1] CameraMovement
  (Pawn|Input|AddControllerYawInput AxisValue))

(event Input|AxisEvents|InputAxisLookUp
  (params (AxisValue :type Float%20%28single-precision%29))
  ;[1 1 1] CameraMovement
  (Pawn|Input|AddControllerPitchInput AxisValue))

(event Input|AxisEvents|InputAxisMoveForward
  (params (AxisValue :type Float%20%28single-precision%29))
  ;[1 1 1] CharacterMovement
  (Pawn|Input|AddMovementInput (Math|Vector|GetForwardVector (Variables|Collision|GetCapsuleComponent)) AxisValue false))

(event Input|AxisEvents|InputAxisMoveRight
  (params (AxisValue :type Float%20%28single-precision%29))
  ;[1 1 1] CharacterMovement
  (Pawn|Input|AddMovementInput (Math|Vector|GetRightVector (Variables|Collision|GetCapsuleComponent)) AxisValue false))

(event Input|KeyboardEvents|NumPadFive
  (params (Key :type Key%20Structure :default "None"))
  ;[1 1 1] Debug Purposes
)

(event Input|KeyboardEvents|NumPadSix
  (params (Key :type Key%20Structure :default "None"))
  ;[1 1 1] Debug Purposes
)

(fn ConstructionScript)

(fn HeightCheck
  (params (B :type Float%20%28double-precision%29))
  (bind _capsulecomponent (Variables|Collision|GetCapsuleComponent))
  (bind _capsulecomponent_2 (Variables|Collision|GetCapsuleComponent))
  (bind _returnvalue (Transformation|GetWorldLocation _capsulecomponent))
  (bind _returnvalue_2 (Transformation|GetWorldLocation _capsulecomponent_2))
  (bind _capsulehalfheight (Variables|/Script/Engine.CapsuleComponent|GetCapsuleHalfHeight _capsulecomponent_2))
  (bind _returnvalue_3 (+ (.z _returnvalue_2) _capsulehalfheight))
  (bind _returnvalue_4 (Math|Vector|MakeVector (.x _returnvalue) (.y _returnvalue) _returnvalue_3))
  (bind (_x _y) (Math|Vector|BreakVector _returnvalue_4))
  (bind _returnvalue_5 (Collision|MultiSphereTraceByChannel _returnvalue_4 (Math|Vector|MakeVector _x _y (+ _returnvalue_3 B)) 2e+01 "TraceTypeQuery1" false 0 "ForDuration"))
  (if _returnvalue_5
    (return false)
    (else
      (return true))))

(fn SetCapsuleHalfHeight
  (params (HalfHeight :type Float%20%28single-precision%29))
  (Components|Capsule|SetCapsuleHalfHeight (Variables|Collision|GetCapsuleComponent) HalfHeight true)
  (Transformation|AddLocalOffset (Variables|Character|GetMesh) "0.000000,0.000000,30.000000" false false))

(fn CrouchMode
  (Variables|Default|SetE_StanceState "NewEnumerator1")
  (Variables|/Script/Engine.CharacterMovementComponent|SetMaxWalkSpeed (Variables|Character|GetCharacterMovement) 1.4e+02))

(fn ProneMode
  (Variables|Default|SetE_StanceState "NewEnumerator2")
  (Variables|/Script/Engine.CharacterMovementComponent|SetMaxWalkSpeed (Variables|Character|GetCharacterMovement) 6e+01))

(fn StandMode
  (bind _canstand_ (CallFunction|HeightCheck 45.0))
  (if _canstand_
    (Variables|Default|SetE_StanceState "NewEnumerator0")
    (Variables|/Script/Engine.CharacterMovementComponent|SetMaxWalkSpeed (Variables|Character|GetCharacterMovement) 3e+02)
    (Transformation|AddLocalOffset (Variables|Character|GetMesh) "0.000000,0.000000,-30.000000" false false)))

(fn PronetoCrouchMode
  (bind _canstand_ (CallFunction|HeightCheck 3e+01))
  (if _canstand_
    (Variables|Default|SetE_StanceState "NewEnumerator1")
    (Variables|/Script/Engine.CharacterMovementComponent|SetMaxWalkSpeed (Variables|Character|GetCharacterMovement) 1.4e+02)
    (Transformation|AddLocalOffset (Variables|Character|GetMesh) "0.000000,0.000000,-30.000000" false false)))