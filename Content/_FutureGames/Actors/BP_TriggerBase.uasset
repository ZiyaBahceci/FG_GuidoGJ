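; BP_TriggerBase is a one-shot trigger that drops a rockfall when the first-person player character enters its TriggerBox.
; The overlap passes a DoOnce into a delayed loop that spawns RocksToFall BP_RockBase actors at random points inside RockFallBox.
; Each spawn also plays a rotational camera shake on the first player's camera.
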(event OnComponentBeginOverlap(TriggerBox)
  (params (OverlappedComponent :type Primitive%20Component%20Object%20Reference) (OtherActor :type Actor%20Object%20Reference) (OtherComp :type Primitive%20Component%20Object%20Reference) (OtherBodyIndex :type Integer) (bFromSweep :type Boolean) (SweepResult :type Hit%20Result%20Structure%20%28by%20ref%29))
  (bind _rockfallbox (Variables|Default|GetRockFallBox))
  (Utilities|Casting|CastToBP_1stPersonCharacter OtherActor)
  (Utilities|FlowControl|DoOnce false
    (:Completed
      (Utilities|ForLoopwithDelay 0 (- (Variables|Default|GetRocksToFall) 1) 0.4
        (:Loop%20Body
          (Game|SpawnActorfromClass "/Game/_FutureGames/Actors/BP_RockBase.BP_RockBase_C" (Math|Transform|MakeTransform (Math|Random|RandomPointinBoundingBox (Transformation|GetWorldLocation _rockfallbox) (Components|Box|GetScaledBoxExtent _rockfallbox)) "0, 0, 0" "1.000000,1.000000,1.000000") "Undefined" "MultiplyWithRoot" 0 0)
          (Class|LegacyCameraShake|StartLegacyCameraShake (Game|GetPlayerCameraManager 0) "/Game/_FutureGames/CameraShake_Rot.CameraShake_Rot_C" 1.0 "CameraLocal" "0, 0, 0"))))))

(fn ConstructionScript)