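; BP_GasMask is a gas mask pickup that the first-person character collects by pressing Interact nearby.
; The actor enables player input, and its Box overlap opens and closes a gate that limits Interact to characters in range.
; On interaction it clears the character's CanBeDamaged flag, waits briefly, sets its own CanBeDamaged, calls PickUpGasMask on the character and destroys itself.
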(event OnComponentBeginOverlap(Box)
  (params (OverlappedComponent :type Primitive%20Component%20Object%20Reference) (OtherActor :type Actor%20Object%20Reference) (OtherComp :type Primitive%20Component%20Object%20Reference) (OtherBodyIndex :type Integer) (bFromSweep :type Boolean) (SweepResult :type Hit%20Result%20Structure%20%28by%20ref%29))
  (bind _asbp_1st_person_character (Utilities|Casting|CastToBP_1stPersonCharacter OtherActor))
  (Utilities|FlowControl|Gate true) ; enters at Open
)

(event OnComponentEndOverlap(Box)
  (params (OverlappedComponent :type Primitive%20Component%20Object%20Reference) (OtherActor :type Actor%20Object%20Reference) (OtherComp :type Primitive%20Component%20Object%20Reference) (OtherBodyIndex :type Integer))
  (Utilities|Casting|CastToBP_1stPersonCharacter OtherActor)
  (Utilities|FlowControl|Gate true) ; enters at Close
)

(event EventBeginPlay
  (Input|EnableInput (Game|GetPlayerController 0)))

(event Input|ActionEvents|InputActionInteract
  (params (Key :type Key%20Structure))
  (:Pressed
    (Utilities|FlowControl|Gate true
      (:Exit
        (Variables|/Script/Engine.Actor|SetbCanBeDamaged (stale OnComponentBeginOverlap(Box) _asbp_1st_person_character) false)
        (Utilities|FlowControl|Delay 0.1)
        (Variables|Actor|SetbCanBeDamaged true)
        (Default|PickUpGasMask (stale OnComponentBeginOverlap(Box) _asbp_1st_person_character))
        (Actor|DestroyActor)))))

(fn ConstructionScript)