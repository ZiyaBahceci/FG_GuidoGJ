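; BP_FlashlightRecharger is a single-use pickup that recharges the first-person character's flashlight battery.
; Its Box overlap caches the BP_1stPersonCharacter and opens a gate that closes when the character leaves.
; With input enabled at BeginPlay, pressing Interact through the open gate calls BatteryRecharge and destroys the actor, unless the battery is already full.
; It also plays a 2D sound at BeginPlay, rather than on pickup.
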(event OnComponentBeginOverlap(Box)
  (params (OverlappedComponent :type Primitive%20Component%20Object%20Reference) (OtherActor :type Actor%20Object%20Reference) (OtherComp :type Primitive%20Component%20Object%20Reference) (OtherBodyIndex :type Integer) (bFromSweep :type Boolean) (SweepResult :type Hit%20Result%20Structure%20%28by%20ref%29))
  (bind _asbp_1st_person_character (Utilities|Casting|CastToBP_1stPersonCharacter OtherActor))
  (Utilities|FlowControl|Gate true) ; enters at Open
)

(event OnComponentEndOverlap(Box)
  (params (OverlappedComponent :type Primitive%20Component%20Object%20Reference) (OtherActor :type Actor%20Object%20Reference) (OtherComp :type Primitive%20Component%20Object%20Reference) (OtherBodyIndex :type Integer))
  (Utilities|Casting|CastToBP_1stPersonCharacter OtherActor)
  (Utilities|FlowControl|Gate true) ; enters at Close
)

(event EventBeginPlay
  (Input|EnableInput (Game|GetPlayerController 0))
  (Audio|PlaySound2D "/Game/_FutureGames/Art/Sound/a/sound.sound" 1.0 1.0 0.0 0 0))

(event Input|ActionEvents|InputActionInteract
  (params (Key :type Key%20Structure))
  (:Pressed
    (Utilities|FlowControl|Gate true
      (:Exit
        (if (not (>= (Variables|/Game/_FutureGames/Actors/BP_1stPersonCharacter.BP_1stPersonCharacter_C|GetBatteryPercent (stale OnComponentBeginOverlap(Box) _asbp_1st_person_character)) 1e+02))
          (Default|BatteryRecharge (stale OnComponentBeginOverlap(Box) _asbp_1st_person_character))
          (Actor|DestroyActor))))))

(fn ConstructionScript)