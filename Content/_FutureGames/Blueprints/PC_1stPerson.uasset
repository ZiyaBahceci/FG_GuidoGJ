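; First-person player controller that toggles the game's pause menu from the Pause input action.
; Pausing creates WBP_PauseMenu, adds it to the viewport, focuses it in Game and UI input mode, shows the cursor and pauses the game.
; Pressing again removes the widget, unpauses and restores game-only input with the cursor hidden.
; BeginPlay sets the controller tickable while paused.
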(event EventTick
  (params (DeltaSeconds :type Float%20%28single-precision%29)))

(event EventBeginPlay
  (Class|Actor|SetTickablewhenPaused self true))

(event Input|ActionEvents|InputActionPause
  (params (Key :type Key%20Structure))
  (bind _self self)
  ;[1 1 1] PauseMenu
  (:Pressed
    (if (not (Variables|Default|GetisPaused?))
      (Variables|Default|SetisPaused? true)
      (bind _returnvalue (UserInterface|CreateWidget "/Game/_FutureGames/Widgets/WBP_PauseMenu.WBP_PauseMenu_C" _self))
      (bind _output_get (Variables|Default|SetPauseMenuWidget _returnvalue))
      (UserInterface|Viewport|AddtoViewport _output_get 15)
      (Input|SetInputModeGameandUI _self (Variables|Default|GetPauseMenuWidget) "DoNotLock" true false)
      (Variables|/Script/Engine.PlayerController|SetbShowMouseCursor self true)
      (Game|SetGamePaused true)
      (else
        (Variables|Default|SetisPaused? false)
        (Widget|RemovefromParent (Variables|Default|GetPauseMenuWidget))
        (Game|SetGamePaused false)
        (Input|SetInputModeGameOnly _self false)
        (Variables|/Script/Engine.PlayerController|SetbShowMouseCursor self false)))))

(fn ConstructionScript)