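; Scripted gas leak trigger actor that plays a leak-to-explosion sequence when its Box is overlapped.
; On BeginPlay it spawns an AF_Wall at its Wall component.
; The overlap chains timed Delays through leak VFX and gas sound, sparks, then a scaled-up explosion with sound, before the actor destroys itself.
; The overlap has no actor filter or once-only guard, so re-entry can replay the leak effect and sound.
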(event OnComponentBeginOverlap(Box)
  (params (OverlappedComponent :type Primitive%20Component%20Object%20Reference) (OtherActor :type Actor%20Object%20Reference) (OtherComp :type Primitive%20Component%20Object%20Reference) (OtherBodyIndex :type Integer) (bFromSweep :type Boolean) (SweepResult :type Hit%20Result%20Structure%20%28by%20ref%29))
  (Niagara|SpawnSystematLocation "/Game/Marcel/Gas_Leak/Leak/NS_Leak.NS_Leak" (Transformation|GetWorldLocation (Variables|Default|GetLeak)))
  (Audio|PlaySound2D "/Game/Marcel/Sound/Gas.Gas" 1.0 1.0 0.0 0 0)
  (Utilities|FlowControl|Delay 1.0)
  (Effects|SpawnEmitteratLocation "/Game/Marcel/Gas_Leak/Spark/PS_Spark.PS_Spark" (Transformation|GetWorldLocation (Variables|Default|GetSparks)))
  (Utilities|FlowControl|Delay 3.0)
  (Effects|SpawnEmitteratLocation "/Game/Marcel/Gas_Leak/P_Explosion.P_Explosion" (Transformation|GetWorldLocation (Variables|Default|GetExplosion)) "0, 0, 0" "10.000000,10.000000,10.000000")
  (Audio|PlaySound2D "/Game/StarterContent/Audio/Explosion_Cue.Explosion_Cue" 1.0 1.0 0.0 0 0)
  (Actor|DestroyActor))

(event EventBeginPlay
  (Game|SpawnActorfromClass "/Game/Ziya/AF_Wall.AF_Wall_C" (Math|Transform|MakeTransform (Transformation|GetWorldLocation (Variables|Default|GetWall)) "0, 0, 0" "1.000000,1.000000,1.000000") "Undefined" "MultiplyWithRoot" 0 0))

(event Collision|EventActorBeginOverlap
  (params (OtherActor :type Actor%20Object%20Reference)))

(event EventTick
  (params (DeltaSeconds :type Float%20%28single-precision%29)))

(fn ConstructionScript)